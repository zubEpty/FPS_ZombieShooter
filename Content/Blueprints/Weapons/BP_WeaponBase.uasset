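; BP_WeaponBase is a weapon Blueprint providing firing, ammo checks and reloading for the player's BP_FPSCharacter, which it caches on BeginPlay.
; Firing spends one round, then line-traces from the camera with random per-axis endpoint spread and debug drawing.
; The trace result is unused, as are the muzzle mesh and socket inputs.
; Reloading sets the magazine from reserve ammo, discarding any rounds still loaded.
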(event EventBeginPlay
  (bind _asbp_fpscharacter (Utilities|Casting|CastToBP_FPSCharacter (Game|Player|GetPlayerPawn 0)))
  (Variables|Default|SetPlayerREF _asbp_fpscharacter))

(fn ConstructionScript)

(fn WeaponFire
  (Variables|Ammo|SetCurrentAmmo (- (Variables|Ammo|GetCurrentAmmo) 1))
  (CallFunction|CalculateShot (Variables|/Game/Blueprints/BP_FPSCharacter.BP_FPSCharacter_C|GetCamera (Variables|Default|GetPlayerREF)) (Variables|Default|GetGunMesh) "MuzzleFlash"))

(fn WeaponReload
  (Variables|Ammo|SetCurrentAmmo (Math|Integer|Min(Integer) (Variables|Ammo|GetMaxMagAmmo) (Variables|Ammo|GetCurrentTotalAmmo)))
  (Variables|Ammo|SetCurrentTotalAmmo (- (Variables|Ammo|GetCurrentTotalAmmo) (Math|Integer|Min(Integer) (Variables|Ammo|GetMaxMagAmmo) (Variables|Ammo|GetCurrentTotalAmmo)))))

(fn HasAmmoinMag
  (return (> (Variables|Ammo|GetCurrentAmmo) 0) (== (Variables|Ammo|GetCurrentAmmo) (Variables|Ammo|GetMaxMagAmmo))))

(fn HasExtraAmmo
  (return (> (Variables|Ammo|GetCurrentTotalAmmo) 0)))

(fn CalculateShot
  (params (Camera :type Camera%20Component%20Object%20Reference) (WeaponMesh :type Scene%20Component%20Object%20Reference) (WeaponFireSocketName :type Name))
  (bind _bulletspread (Variables|Properties|GetBulletSpread))
  (bind _returnvalue (* _bulletspread -1.0))
  (Utilities|FlowControl|Sequence
    (:then_0
      (LocalVariables|SetLocalCamera Camera)
      (LocalVariables|SetLocalWeaponMesh WeaponMesh)
      (LocalVariables|SetLocalSocketName WeaponFireSocketName))
    (:then_1
      (Collision|LineTraceForObjects (.location (Transformation|GetWorldTransform (LocalVariables|GetLocalCamera))) (Math|Vector|MakeVector (+ (.X (Math|Vector|BreakVector (+ (.location (Transformation|GetWorldTransform (LocalVariables|GetLocalCamera))) (* (Math|Vector|GetForwardVector (.rotation (Transformation|GetWorldTransform (LocalVariables|GetLocalCamera)))) 1e+04)))) (Math|Random|RandomFloatinRange _returnvalue _bulletspread)) (+ (.Y (Math|Vector|BreakVector (+ (.location (Transformation|GetWorldTransform (LocalVariables|GetLocalCamera))) (* (Math|Vector|GetForwardVector (.rotation (Transformation|GetWorldTransform (LocalVariables|GetLocalCamera)))) 1e+04)))) (Math|Random|RandomFloatinRange _returnvalue _bulletspread)) (+ (.Z (Math|Vector|BreakVector (+ (.location (Transformation|GetWorldTransform (LocalVariables|GetLocalCamera))) (* (Math|Vector|GetForwardVector (.rotation (Transformation|GetWorldTransform (LocalVariables|GetLocalCamera)))) 1e+04)))) (Math|Random|RandomFloatinRange _returnvalue _bulletspread))) (Utilities|Array|MakeArray "ObjectTypeQuery1" "ObjectTypeQuery2") false (Utilities|Array|MakeArray (Game|Player|GetPlayerPawn 0)) "ForDuration"))))